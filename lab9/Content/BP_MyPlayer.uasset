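; BP_MyPlayer is a player pawn Blueprint that provides basic movement and mouse look.
; Each Tick, a sequence polls W, A, S and D on player controller 0 directly and adds movement input along the actor's forward or right vector.
; MouseX and MouseY axis events drive controller yaw and pitch, with the vertical axis inverted by negation.
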(event `self.ReceiveTick`
  (params (DeltaSeconds :type "Float (single-precision)"))
  (bind _returnvalue (`GameplayStatics.GetPlayerController` 0))
  (`|ExecutionSequence`
    (:`then_0`
      (if (`PlayerController.IsInputKeyDown` _returnvalue "W")
        (`self.AddMovementInput` (`self.GetActorForwardVector`))))
    (:`then_1`
      (if (`PlayerController.IsInputKeyDown` _returnvalue "S")
        (`self.AddMovementInput` (`self.GetActorForwardVector`) -1.0)))
    (:`then_2`
      (if (`PlayerController.IsInputKeyDown` _returnvalue "A")
        (`self.AddMovementInput` (`self.GetActorRightVector`) -1.0)))
    (:`then_3`
      (if (`PlayerController.IsInputKeyDown` _returnvalue "D")
        (`self.AddMovementInput` (`self.GetActorRightVector`))))))

(event `InputAxisKey|MouseX`
  (params (AxisValue :type "Float (single-precision)"))
  (`self.AddControllerYawInput` AxisValue))

(event `InputAxisKey|MouseY`
  (params (AxisValue :type "Float (single-precision)"))
  (`self.AddControllerPitchInput` (* AxisValue -1.0)))

(fn `UserConstructionScript`)